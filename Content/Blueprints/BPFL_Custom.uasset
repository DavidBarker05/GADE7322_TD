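; Blueprint function library that defines team attitudes (Friendly, Hostile, Neutral) between defender and attacker roles.
; GetAttitudeCustom holds a switch on TeamA into three sub-graphs that switch on TeamB: Attackers, Melee Defender, and Ranged and Support Defenders.
; Same side is Friendly and opposing sides Hostile, except Melee Defenders are Neutral toward Flying Attackers.
; The function entry is unwired, so this logic never runs.
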(fn `GetAttitudeCustom`
  (params (`Team A` :type "EAITeam Enum" :default "MeleeDefender") (`Team B` :type "EAITeam Enum" :default "MeleeDefender"))
  (returns (Attitude :type "ETeamAttitude Enum"))
  (locals (`Result Attitude` :type "ETeamAttitude Enum")))